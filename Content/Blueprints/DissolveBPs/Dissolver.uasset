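; Dissolver actor that feeds the position and size of its CubicDissolver component to materials as a dissolve volume.
; SetDissolverMatParameters writes the component's world location and scale into the DissolveLocation and BoundsVector parameters of MPC_DissolveMatParameters.
; It runs from the construction script and every Tick, so materials reading the shared collection follow the volume as it changes.
; Rotation is not passed, and SetDissolverParameters is an empty stub.
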(event `self.ReceiveTick`
  (params (DeltaSeconds :type "Float (single-precision)"))
  (`self.SetDissolverMatParameters`))

(fn `SetDissolverMatParameters`
  (bind _cubicdissolver (`self.CubicDissolver`))
  (`KismetMaterialLibrary.SetVectorParameterValue` "/Game/Materials/Dissolve_Material/MPC_DissolveMatParameters.MPC_DissolveMatParameters" "DissolveLocation" (`KismetMathLibrary.Conv_VectorToLinearColor` (`SceneComponent.K2_GetComponentLocation` _cubicdissolver)))
  (`KismetMaterialLibrary.SetVectorParameterValue` "/Game/Materials/Dissolve_Material/MPC_DissolveMatParameters.MPC_DissolveMatParameters" "BoundsVector" (`KismetMathLibrary.Conv_VectorToLinearColor` (`SceneComponent.K2_GetComponentScale` _cubicdissolver))))

(fn `SetDissolverParameters`)

(fn `UserConstructionScript`
  (`self.SetDissolverMatParameters`))