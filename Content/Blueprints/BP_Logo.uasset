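; BP_Logo is a logo actor that feeds a dissolve volume to materials and exposes a transparency control for its plane mesh.
; On construction and every tick, it writes the DissolverCubeActor's location and scale into MPC_DissolveParam2 as dissolve center and bounds.
; Without a valid cube, it prints a warning and writes zero vectors.
; MeshTransparencyEvent sets the Plane material's opacity parameter and prints the value.
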(event `self.ReceiveTick`
  (params (DeltaSeconds :type "Float (single-precision)"))
  (`self.SetMPCValues`))

(event `MeshTransparencyEvent`
  (params (val :type "Float (double-precision)"))
  (`self.SetLogoMatParam` val))

(fn `SetLogoMatParam`
  (params (val :type "Float (double-precision)"))
  (`MeshComponent.SetScalarParameterValueOnMaterials` (`self.Plane`) "Opacity_value" val)
  (`KismetSystemLibrary.PrintString` (`KismetStringLibrary.Conv_DoubleToString` val)))

(fn `SetMPCValues`
  (bind _dissolvercubeactor (`self.DissolverCubeActor`))
  (`/Engine/EditorBlueprintResources/StandardMacros.IsValid` _dissolvercubeactor
    (:`Is Valid`
      (set `self.DissolveLocation` (`self.K2_GetActorLocation` _dissolvercubeactor))
      (set `self.DissolveBoundsVector` (`self.GetActorScale3D` _dissolvercubeactor)))
    (:`Is Not Valid`
      (`KismetSystemLibrary.PrintString` "Dissolver mesh not set")
      (set `self.DissolveLocation` (0.0 0.0 0.0))
      (set `self.DissolveBoundsVector` (0.0 0.0 0.0))))
  (`KismetMaterialLibrary.SetVectorParameterValue` "/Game/Materials/Dissolve_Material/MPC_DissolveParam2.MPC_DissolveParam2" "DissolveLocation" (`KismetMathLibrary.Conv_VectorToLinearColor` (`self.DissolveLocation`)))
  (`KismetMaterialLibrary.SetVectorParameterValue` "/Game/Materials/Dissolve_Material/MPC_DissolveParam2.MPC_DissolveParam2" "BoundsVector" (`KismetMathLibrary.Conv_VectorToLinearColor` (`self.DissolveBoundsVector`))))

(fn `UserConstructionScript`
  (`self.SetMPCValues`))