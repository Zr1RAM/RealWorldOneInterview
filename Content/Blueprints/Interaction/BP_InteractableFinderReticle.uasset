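; Interaction reticle actor that finds, highlights, selects and rotates Interactable actors from the player's view.
; Each tick a visibility trace along the player pawn's camera forward vector tracks the current Interactable and toggles its highlight.
; Holding left mouse selects it, pausing tracing and camera rotation and notifying the HUD until release.
; Holding right mouse rotates the current Interactable by mouse delta.
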(event `self.ReceiveBeginPlay`
  (`self.Initialization`))

(event `self.ReceiveTick`
  (params (DeltaSeconds :type "Float (single-precision)"))
  (`self.InteractablePointer`)
  (`self.RotateInteractable`))

(event `InputAction|LMB`
  (params (Key :type "Key Structure"))
  (:`Pressed`
    (`self.ToggleSelectionOfInteractable` true))
  (:`Released`
    (`self.ToggleSelectionOfInteractable` false)))

(event `InputAction|RMB`
  (params (Key :type "Key Structure"))
  (:`Pressed`
    (set `self.CanRotateInteractable` true))
  (:`Released`
    (set `self.CanRotateInteractable` false)))

(fn `Initialization`
  (`|ExecutionSequence`
    (:`then_0`
      (bind _ascharacter_pawn (cast `/Game/Blueprints/Base/CharacterPawn` (`GameplayStatics.GetPlayerPawn` 0)))
      (set `self.PlayerCamera` (`self.GetComponentByClass` _ascharacter_pawn "/Script/Engine.CameraComponent")))))

(fn `Interactable Line Tracer`
  (bind _playercamera (`self.PlayerCamera`))
  (bind _currentinteractable (`self.CurrentInteractable`))
  (bind _returnvalue (`SceneComponent.K2_GetComponentLocation` _playercamera))
  (if (`self.isLineTracing`)
    (bind (_outhit _returnvalue_2) (`KismetSystemLibrary.LineTraceSingle` :`Start` _returnvalue :`End` (+ _returnvalue (* (`SceneComponent.GetForwardVector` _playercamera) (`self.MaxTraceDistance`))) :`TraceChannel` "TraceTypeQuery1" :`DrawDebugType` "ForOneFrame"))
    (if _returnvalue_2
      (bind _asinteractable (cast `/Game/Blueprints/Interaction/Interactable` (`.HitActor` (`GameplayStatics.BreakHitResult` _outhit)))
        (:`then`
          (bind _output_get (set `self.CurrentInteractable` _asinteractable))
          (`/Game/Blueprints/Interaction/Interact_Interface.OnHighlightInteractable` _output_get))
        (:`CastFailed`
          (`/Engine/EditorBlueprintResources/StandardMacros.IsValid` _currentinteractable
            (:`Is Valid`
              (`/Game/Blueprints/Interaction/Interact_Interface.OnUnhighlightInteractable` _currentinteractable)
              (set `self.CurrentInteractable` null))))))))

(fn `InteractablePointer`
  (`self.Interactable Line Tracer`))

(fn `RotateInteractable`
  (bind _currentinteractable (`self.CurrentInteractable`))
  (bind (_deltax _deltay) (`PlayerController.GetInputMouseDelta` (`GameplayStatics.GetPlayerController` 0)))
  (if (`self.CanRotateInteractable`)
    (`/Engine/EditorBlueprintResources/StandardMacros.IsValid` _currentinteractable
      (:`Is Valid`
        (`self.K2_AddActorWorldRotation` _currentinteractable (`KismetMathLibrary.MakeRotator` 0.0 (* _deltay -1.0) (* _deltax -1.0)) false false)))))

(fn `ToggleSelectionOfInteractable`
  (params (isSelected :type Boolean))
  (bind _currentinteractable (`self.CurrentInteractable`))
  (bind _returnvalue (`PlayerController.GetHUD` (`GameplayStatics.GetPlayerController` 0)))
  (`/Engine/EditorBlueprintResources/StandardMacros.IsValid` _currentinteractable
    (:`Is Valid`
      (bind _ascharacter_pawn (cast `/Game/Blueprints/Base/CharacterPawn` (`GameplayStatics.GetPlayerPawn` 0)))
      (bind _output_get (set `/Game/Blueprints/Base/CharacterPawn.IsCameraRotationActive` (not isSelected) _ascharacter_pawn))
      (bind _output_get_2 (set `self.isLineTracing` _output_get))
      (if _output_get_2
        (`/Game/Blueprints/Interaction/Interactable.OnDeselectInteractable` _currentinteractable)
        (message `/Game/Blueprints/Interaction/Interact_Interface.OnDeselectInteractable` _returnvalue)
        (else
          (`/Game/Blueprints/Interaction/Interactable.OnSelectIntereactable` _currentinteractable)
          (message `/Game/Blueprints/Interaction/Interact_Interface.OnSelectIntereactable` _returnvalue))))))

(fn `UserConstructionScript`)