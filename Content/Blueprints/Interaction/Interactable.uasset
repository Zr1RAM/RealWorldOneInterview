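; Base interactable actor that the player can highlight and pick up for inspection in front of the camera.
; Highlighting toggles an outline through the mesh's custom depth stencil, using a mesh supplied via SetInteractableMeshComp, which also records the original transform.
; Selection sets a destination ahead of the CharacterPawn camera, and deselection restores the original location.
; Tick lerps location toward the destination and eases rotation back whenever unselected.
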(event `self.ReceiveTick`
  (params (DeltaSeconds :type "Float (single-precision)"))
  (`self.LerpItemLocation`)
  (`self.LerpBackItemRotation`))

(event `/Game/Blueprints/Interaction/Interact_Interface.OnHighlightInteractable`
  (`self.ToggleBorder` true))

(event `/Game/Blueprints/Interaction/Interact_Interface.OnUnhighlightInteractable`
  (`self.ToggleBorder` false))

(event `/Game/Blueprints/Interaction/Interact_Interface.OnSelectIntereactable`
  (bind _ascharacter_pawn (cast `/Game/Blueprints/Base/CharacterPawn` (`GameplayStatics.GetPlayerPawn` 0)))
  (bind _returnvalue (`self.GetComponentByClass` _ascharacter_pawn "/Script/Engine.CameraComponent"))
  (set `self.DestinationLocation` (+ (`SceneComponent.K2_GetComponentLocation` _returnvalue) (* (`SceneComponent.GetForwardVector` _returnvalue) (`self.OffsetDistanceFromPlayerPawn`))))
  (set `self.isLerpingLocation` true)
  (set `self.isSelected` true)
  (`self.ToggleBorder` false))

(event `/Game/Blueprints/Interaction/Interact_Interface.OnDeselectInteractable`
  (set `self.DestinationLocation` (`self.ItemInitialLocation`))
  (set `self.isLerpingLocation` true)
  (set `self.isSelected` false))

(fn `LerpBackItemRotation`
  (if (not (`self.isSelected`))
    (`self.K2_SetActorRotation` (`KismetMathLibrary.RLerp` (`self.K2_GetActorRotation`) (`self.OriginalRotation`) 0.2) true)))

(fn `LerpItemLocation`
  (if (`self.isLerpingLocation`)
    (`self.K2_SetActorLocation` (`KismetMathLibrary.VLerp` (`self.K2_GetActorLocation`) (`self.DestinationLocation`) (* (`GameplayStatics.GetWorldDeltaSeconds`) (`self.LerpingSpeed`))) false true)
    (if (<= (`KismetMathLibrary.Vector_Distance` (`self.K2_GetActorLocation`) (`self.DestinationLocation`)) 0.1)
      (set `self.isLerpingLocation` false)
      (`self.K2_SetActorLocation` (`self.DestinationLocation`) false true))))

(fn `MakeMeshInteractable`
  (`PrimitiveComponent.SetRenderCustomDepth` (`self.InteractableStaticMeshComp`) true)
  (set `self.ItemInitialLocation` (`self.K2_GetActorLocation`))
  (set `self.OriginalRotation` (`self.K2_GetActorRotation`)))

(fn `SetInteractableMeshComp`
  (params (Mesh :type "StaticMeshComponent Object Reference"))
  (set `self.InteractableStaticMeshComp` Mesh)
  (`self.MakeMeshInteractable`))

(fn `ToggleBorder`
  (params (Val :type Boolean))
  (bind _interactablestaticmeshcomp (`self.InteractableStaticMeshComp`))
  (if Val
    (`PrimitiveComponent.SetCustomDepthStencilValue` _interactablestaticmeshcomp 2)
    (else
      (`PrimitiveComponent.SetCustomDepthStencilValue` _interactablestaticmeshcomp 0))))

(fn `UserConstructionScript`)