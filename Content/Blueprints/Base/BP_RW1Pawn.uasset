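; BP_RW1Pawn is a player-controlled pawn with basic axis-driven movement and mouse look.
; MoveForward and MoveRight add movement input along the actor's forward and right vectors.
; Turn and LookUp feed controller yaw and pitch, scaled by the MouseSpeed variable.
; MoveForward also prints its axis value on screen as debug output, and the construction script is empty.
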(event `InputAxis|MoveForward`
  (params (AxisValue :type "Float (single-precision)"))
  (`self.AddMovementInput` (`self.GetActorForwardVector`) AxisValue)
  (`KismetSystemLibrary.PrintString` (`KismetStringLibrary.Conv_DoubleToString` AxisValue) true true (struct :`G` 0.66 :`B` 1.0 :`A` 1.0) 0.2))

(event `InputAxis|Turn`
  (params (AxisValue :type "Float (single-precision)"))
  (`self.AddControllerYawInput` (* AxisValue (`self.MouseSpeed`))))

(event `InputAxis|MoveRight`
  (params (AxisValue :type "Float (single-precision)"))
  (`self.AddMovementInput` (`self.GetActorRightVector`) AxisValue))

(event `InputAxis|LookUp`
  (params (AxisValue :type "Float (single-precision)"))
  (`self.AddControllerPitchInput` (* AxisValue (`self.MouseSpeed`))))

(fn `UserConstructionScript`)