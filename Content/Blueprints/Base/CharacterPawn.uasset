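; Base player pawn that handles axis input for first-person-style movement and camera look.
; Forward and right axes move the pawn itself, while turn and look-up inputs, scaled by MouseSpeed, rotate PawnToControl, which is set to self on BeginPlay.
; Movement and rotation are gated by multiplying input by boolean flags, both switched through PlayerMovementToggleEvent and ToggleCharacterControls.
; SetPawnToControl is an empty stub.
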(event `self.ReceiveBeginPlay`
  (set `self.PawnToControl` self))

(event `InputAxis|MoveForward`
  (params (AxisValue :type "Float (single-precision)"))
  ;[1 1 1] Player Camera Movement
  (`self.AddMovementInput` (`self.GetActorForwardVector`) (* AxisValue (`KismetMathLibrary.Conv_BoolToDouble` (`self.isPawnMoveable`)))))

(event `InputAxis|Turn`
  (params (AxisValue :type "Float (single-precision)"))
  ;[1 1 1] Player Camera Rotation
  (`self.AddControllerYawInput` (`self.PawnToControl`) (* AxisValue (`self.MouseSpeed`) (`KismetMathLibrary.Conv_BoolToDouble` (`self.IsCameraRotationActive`)))))

(event `InputAxis|MoveRight`
  (params (AxisValue :type "Float (single-precision)"))
  ;[1 1 1] Player Camera Movement
  (`self.AddMovementInput` (`self.GetActorRightVector`) (* AxisValue (`KismetMathLibrary.Conv_BoolToDouble` (`self.isPawnMoveable`)))))

(event `InputAxis|LookUp`
  (params (AxisValue :type "Float (single-precision)"))
  ;[1 1 1] Player Camera Rotation
  (`self.AddControllerPitchInput` (`self.PawnToControl`) (* AxisValue (`self.MouseSpeed`) (`KismetMathLibrary.Conv_BoolToDouble` (`self.IsCameraRotationActive`)))))

(event `PlayerMovementToggleEvent`
  (params (Val :type Boolean))
  (`self.ToggleCharacterControls` Val))

(fn `SetPawnToControl`
  (params (PawnToControl :type "Pawn Object Reference")))

(fn `ToggleCharacterControls`
  (params (Val :type Boolean))
  (bind _output_get (set `self.isPawnMoveable` Val))
  (set `self.IsCameraRotationActive` _output_get))

(fn `UserConstructionScript`)